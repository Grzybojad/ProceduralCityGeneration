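; BP_CityGenerator procedurally builds a city from a seed.
; GenerateCity seeds its generators, then builds a road graph using either a Voronoi or an agent-based method, selected by a toggle, with optional debug drawing.
; The resulting road paths feed a spline road generator, while building plots feed a building mesh generator, which destroys its spawned meshes when buildings are disabled.
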(fn ConstructionScript)

(fn GenerateCity
  (bind _buildinggenerator (Variables|Default|GetBuildingGenerator))
  (CallFunction|SetSeed)
  (bind (_road_paths _building_plots) (CallFunction|GenerateRoadNetwork))
  (Class|SplineRoadsGenerator|GenerateRoads (Variables|Default|GetSplineRoadsGenerator) _road_paths)
  (if (Variables|Default|GetGenerateBuildings)
    (Class|BuildingGenerator|GenerateBuildingMeshesfromBuildingPlots _buildinggenerator _building_plots)
    (else
      (Class|BuildingGenerator|DestroySpawnedMeshes _buildinggenerator))))

(fn SetSeed
  (Class|RoadGraphVoronoi|SetSeed (Variables|Default|GetRoadGraphVoronoi) (Variables|Default|GetSeed))
  (Class|RoadGraphAgents|SetSeed (Variables|Default|GetRoadGraphAgents) (Variables|Default|GetSeed))
  (Class|BuildingGenerator|SetSeed (Variables|Default|GetBuildingGenerator) (Variables|Default|GetSeed)))

(fn GenerateRoadNetwork
  (bind _roadgraphvoronoi (Variables|Default|GetRoadGraphVoronoi))
  (bind _roadgraphagents (Variables|Default|GetRoadGraphAgents))
  (Rendering|Debug|FlushPersistentDebugLines)
  (if (Variables|Default|GetVoronoi)
    (Class|RoadGraphVoronoi|GenerateRoadNetwork _roadgraphvoronoi) ; Voronoi Road Graph
    (if (Variables|Default|GetDrawRoadDebug)
      (Class|RoadGraphVoronoi|DrawDebugGraph (Variables|Default|GetRoadGraphVoronoi)))
    (return (Class|RoadGraphVoronoi|GetRoadPaths _roadgraphvoronoi) (Class|RoadGraphVoronoi|GetBuildingPlots _roadgraphvoronoi))
    (else
      (Class|RoadGraphAgents|GenerateRoadNetwork _roadgraphagents) ; Agent Road Graph
      (if (Variables|Default|GetDrawRoadDebug)
        (Class|RoadGraphAgents|DrawDebugGraph (Variables|Default|GetRoadGraphAgents)))
      (return (Class|RoadGraphAgents|GetRoadPaths _roadgraphagents) (Class|RoadGraphAgents|GetBuildingPlots _roadgraphagents)))))