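; Terrain generator Blueprint that builds a procedural mesh landscape at BeginPlay from seeded noise.
; It creates a Diamond-Square or Perlin heightmap, remaps it through a height curve, then converts it into vertices, triangles and UVs for the mesh.
; A visualizer setting can replace the material with a dynamic instance showing a heightmap or incline texture, with UVs rescaled by grid width.
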(event EventBeginPlay
  (CallFunction|GenerateTerrain))

(fn ConstructionScript)

(fn GenerateTerrain
  (LocalVariables|SetHeightmap (Class|TerrainMeshLibrary|RemapHeightmapValues (CallFunction|GetHeightmap) (Variables|Default|GetXSize) (Variables|Default|GetYSize) (Variables|Default|GetHeightCurve)))
  (Class|TerrainMeshLibrary|GenerateTerrainMesh (Variables|Default|GetProceduralMesh) (Variables|Default|GetMaterial) (.Vertices (CallFunction|GenerateTerrainDatafromHeightmap (LocalVariables|GetHeightmap) (Variables|Default|GetXSize) (Variables|Default|GetYSize) (CallFunction|GettheRightUVScale))) (.Triangles (CallFunction|GenerateTerrainDatafromHeightmap (LocalVariables|GetHeightmap) (Variables|Default|GetXSize) (Variables|Default|GetYSize) (CallFunction|GettheRightUVScale))) (.UV0 (CallFunction|GenerateTerrainDatafromHeightmap (LocalVariables|GetHeightmap) (Variables|Default|GetXSize) (Variables|Default|GetYSize) (CallFunction|GettheRightUVScale))))
  (if (CallFunction|ShouldShowSpecialTexture)
    (CallFunction|SetSpecialTerrainTexture (LocalVariables|GetHeightmap) (Variables|Default|GetXSize) (Variables|Default|GetYSize))))

(fn SetSpecialTerrainTexture
  (params (HeightmapValues :type Array%20of%20Floats%20%28single-precision%29) (XSize :type Integer) (YSize :type Integer))
  (switch Utilities|FlowControl|Switch|SwitchonTerrainVisualizationMode (Variables|/Game/_ProcGen/Blueprints/BP_TerrainGenerator_Visualizator.BP_TerrainGenerator_Visualizator_C|GetVisualization (Variables|Default|GetBP_TerrainGenerator_Visualizator))
    (:NewEnumerator1
      (bind _returnvalue (Class|TerrainVisualization|HeightmaptoTexture HeightmapValues XSize YSize))
      (CallFunction|SetCustomTexture _returnvalue))
    (:NewEnumerator2
      (bind _returnvalue_2 (Class|TerrainVisualization|HeightmaptoInclineTexture HeightmapValues XSize YSize))
      (CallFunction|SetCustomTexture _returnvalue_2))))

(fn GettheRightUVScale
  (return (Math|Float|SelectFloat (/ 1.0 (Math|Conversions|ToFloat(Integer) (Variables|Default|GetXSize))) (Variables|Default|GetUVScale) (CallFunction|ShouldShowSpecialTexture))))

(fn ShouldShowSpecialTexture
  (return (Utilities|Enum|NotEqual(Enum) (Variables|/Game/_ProcGen/Blueprints/BP_TerrainGenerator_Visualizator.BP_TerrainGenerator_Visualizator_C|GetVisualization (Variables|Default|GetBP_TerrainGenerator_Visualizator)) "NewEnumerator0")))

(fn SetCustomTexture
  (params (Texture :type Texture%202D%20Object%20Reference))
  (bind _returnvalue (Rendering|Material|CreateDynamicMaterialInstance (Variables|Default|GetProceduralMesh) 0 "/Game/_ProcGen/M_TerrainMaterial.M_TerrainMaterial" "None" :!class /Script/Engine.PrimitiveComponent))
  (Rendering|Material|SetTextureParameterValue _returnvalue "Texture" Texture)
  (Rendering|Material|SetMaterial (Variables|Default|GetProceduralMesh) 0 _returnvalue))

(fn GenerateTerrainDatafromHeightmap
  (params (Heightmap :type Array%20of%20Floats%20%28double-precision%29) (XSize :type Integer) (YSize :type Integer) (UVScale :type Float%20%28double-precision%29))
  (bind _zmultiplier (Variables|Default|GetZMultiplier))
  (bind _vertexdistance (Variables|Default|GetVertexDistance))
  (bind (_vertices _triangles _uv0) (Class|TerrainMeshLibrary|HeightmaptoMesh Heightmap XSize YSize _vertexdistance _zmultiplier UVScale))
  (return _vertices _triangles _uv0))

(fn GetHeightmap
  (if (Variables|Default|GetDiamondSquare)
    (Class|DiamondSquareNoiseGenerator|SetSeed (Variables|Default|GetDiamondSquareNoiseGenerator) (Variables|Default|GetSeed))
    (return (Class|DiamondSquareNoiseGenerator|DiamondSquareHeightmap (Variables|Default|GetDiamondSquareNoiseGenerator) (Variables|Default|GetXSize)))
    (else
      (Class|PerlinNoiseGenerator|SetSeed (Variables|Default|GetPerlinNoiseGenerator) (Variables|Default|GetSeed))
      (return (Class|PerlinNoiseGenerator|PerlinNoiseHeightmap (Variables|Default|GetPerlinNoiseGenerator) (Variables|Default|GetXSize) (Variables|Default|GetYSize))))))